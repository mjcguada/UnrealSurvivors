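; BP_Gem is a gem pickup that homes in on the player and disappears on contact.
; Tick checks the distance to player 0 until it is within MinDistance, then latches PlayerFound and interpolates toward the player every frame without sweeping.
; A trailing Delay in the out-of-range branch has nothing after it, so the check still runs each frame.
; Capsule overlap with BP_Player destroys the gem, with no reward logic here.
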(event OnComponentBeginOverlap(Capsule)
  (params (OverlappedComponent :type Primitive%20Component%20Object%20Reference) (OtherActor :type Actor%20Object%20Reference) (OtherComp :type Primitive%20Component%20Object%20Reference) (OtherBodyIndex :type Integer) (bFromSweep :type Boolean) (SweepResult :type Hit%20Result%20Structure%20%28by%20ref%29))
  ;[1 1 1] Destroy Gem when colliding with the player
  (Utilities|Casting|CastToBP_Player OtherActor)
  (Actor|DestroyActor))

(event EventTick
  (params (DeltaSeconds :type Float%20%28single-precision%29))
  (if (Variables|Default|GetPlayerFound)
    (Transformation|SetActorLocation (Math|Interpolation|VInterpTo (.location (Transformation|GetActorTransform)) (Transformation|GetActorLocation (Game|GetPlayerCharacter 0)) (Utilities|Time|GetWorldDeltaSeconds) 2.0) false false)
    (elif (<= (Transformation|GetDistanceTo (Game|GetPlayerCharacter 0)) (Variables|Default|GetMinDistance))
      (Variables|Default|SetPlayerFound true)
      (else
        (Utilities|FlowControl|Delay 0.2)))))

(fn ConstructionScript)