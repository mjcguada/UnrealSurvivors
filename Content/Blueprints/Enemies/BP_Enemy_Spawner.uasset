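; Enemy spawner actor that repeatedly spawns waves of a configurable enemy class at its own transform, starting on BeginPlay.
; A custom event loops over the enemy count, with a Frequency delay placed before each spawn call inside the loop.
; After the loop, it waits SpawnDelay and calls itself again with the current actor transform, repeating with no stop condition.
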(event Custom|Spawn_Enemy
  (params (EnemyClass :type Actor%20Class%20Reference) (SpawnTransform :type Transform) (NumberOfEnemies :type Integer) (Frequency :type Float%20%28single-precision%29))
  (for _index (range 1 NumberOfEnemies)
    (Utilities|FlowControl|Delay Frequency)
    (Game|SpawnActorfromClass EnemyClass SpawnTransform "Undefined" 0 0))
  ;[1 1 1] After finishing, we call the function again
  (Utilities|FlowControl|Delay (Variables|Default|GetSpawnDelay))
  (CallFunction|SpawnEnemy (Variables|Default|GetEnemy%20Class) (Transformation|GetActorTransform) (Variables|Default|GetNumber%20Of%20Enemies) (Variables|Default|GetFrequency)))

(event EventBeginPlay
  (CallFunction|SpawnEnemy (Variables|Default|GetEnemy%20Class) (Transformation|GetActorTransform) (Variables|Default|GetNumber%20Of%20Enemies) (Variables|Default|GetFrequency)))

(fn ConstructionScript)