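; BP_BasicEnemy is a Paper2D skeleton enemy that hurts the player on contact and drops a gem when killed.
; Each tick it flips its rotation to match its horizontal velocity.
; Its box overlap damages BP_Player, or applies damage to itself when hit by BP_Projectile.
; AnyDamage reduces Health, then either spawns BP_Gem and destroys the enemy or briefly plays a hit flipbook before restoring the walk animation.
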(event OnComponentBeginOverlap(Box)
  (params (OverlappedComponent :type Primitive%20Component%20Object%20Reference) (OtherActor :type Actor%20Object%20Reference) (OtherComp :type Primitive%20Component%20Object%20Reference) (OtherBodyIndex :type Integer) (bFromSweep :type Boolean) (SweepResult :type Hit%20Result%20Structure%20%28by%20ref%29))
  (Utilities|FlowControl|Sequence
    (:then_0
      (bind _asbp_player (Utilities|Casting|CastToBP_Player OtherActor))
      (Game|Damage|ApplyDamage _asbp_player 1e+01 0 0 "/Script/Engine.DamageType"))
    (:then_1
      (Utilities|Casting|CastToBP_Projectile OtherActor)
      (Game|Damage|ApplyDamage self 1.0 0 0))))

(event Custom|UpdateOrientation
  ;[1 1 1] FaceOrientation
  (if (> (.X (Class|KismetMathLibrary|BreakVector3f (Transformation|GetVelocity))) 0.0)
    (Transformation|SetActorRotation "0, 0, 0")
    (else
      (Transformation|SetActorRotation "0.000000,180.000000,0.000000"))))

(event EventBeginPlay)

(event Collision|EventActorBeginOverlap
  (params (OtherActor :type Actor%20Object%20Reference)))

(event EventTick
  (params (DeltaSeconds :type Float%20%28single-precision%29))
  ;[1 1 1] Update()
  (CallFunction|UpdateOrientation))

(event Game|Damage|EventAnyDamage
  (params (Damage :type Float%20%28single-precision%29) (DamageType :type Damage%20Type%20Object%20Reference) (InstigatedBy :type Controller%20Object%20Reference) (DamageCauser :type Actor%20Object%20Reference))
  (bind _output_get (Variables|Default|SetHealth (- (Variables|Default|GetHealth) Damage)))
  (if (<= _output_get 0.0)
    (bind _returnvalue (Game|SpawnActorfromClass "/Game/Blueprints/Items/BP_Gem.BP_Gem_C" (Transformation|GetActorTransform) "Undefined" 0 0))
    (Transformation|SetActorRotation _returnvalue)
    (Actor|DestroyActor)
    (else
      (Sprite|SetFlipbook (Variables|Default|GetSprite) "/Game/Images/sprites/Skeleton/Skeleton_Hit1.Skeleton_Hit1")
      (Utilities|FlowControl|Delay (Class|PaperFlipbookComponent|GetFlipbookLength (Variables|Default|GetSprite)))
      (Sprite|SetFlipbook (Variables|Default|GetSprite) "/Game/Images/sprites/Skeleton/FB_SkeletonWalk.FB_SkeletonWalk"))))

(fn ConstructionScript)