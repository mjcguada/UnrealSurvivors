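; Blueprint function library with a helper that finds the actor of a given class nearest to a supplied player location.
; It gets all actors of that class and loops through them, tracking the closest in local variables.
; Distance is measured in 2D, so height is ignored.
; It returns the nearest actor and its distance.
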(fn FindNearestActorOfClass
  (params (Class :type Actor%20Class%20Reference) (PlayerLocation :type Vector))
  (bind _outactors (Actor|GetAllActorsOfClass 0 Class))
  (for _array_element _outactors
    (if (< (Math|Vector|Distance2D(Vector) (Math|Conversions|ToVector2D(Vector) (Transformation|GetActorLocation _array_element)) (Math|Conversions|ToVector2D(Vector) PlayerLocation)) (LocalVariables|GetLocal_NearestDistance))
      (LocalVariables|SetLocal_NearestDistance (Math|Vector|Distance2D(Vector) (Math|Conversions|ToVector2D(Vector) (Transformation|GetActorLocation _array_element)) (Math|Conversions|ToVector2D(Vector) PlayerLocation)))
      (LocalVariables|SetLocal_NearestActor _array_element)))
  (return (LocalVariables|GetLocal_NearestActor) (LocalVariables|GetLocal_NearestDistance)))