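; Player character with flipbook animation that auto-fires at enemies, collects gems and extends the world as it moves.
; A looping timer aims at the nearest pooled enemy, gating a recursive delayed burst-fire loop.
; Tick updates sprite and facing, spins an attack axis, and traces down ahead of movement to request missing floor from BP_WorldGenerator.
; Gem overlaps raise score toward a doubling threshold; damage uses an invulnerability cooldown, subtracting health after the delay.
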(event OnComponentBeginOverlap(CapsuleComponent)
  (params (OverlappedComponent :type Primitive%20Component%20Object%20Reference) (OtherActor :type Actor%20Object%20Reference) (OtherComp :type Primitive%20Component%20Object%20Reference) (OtherBodyIndex :type Integer) (bFromSweep :type Boolean) (SweepResult :type Hit%20Result%20Structure%20%28by%20ref%29))
  (bind _asbp_gem (Utilities|Casting|CastToBP_Gem OtherActor))
  (Utilities|FlowControl|Sequence
    (:then_0
      (Variables|Default|SetScore (+ (Variables|Default|GetScore) 1.0))
      (if (== (Variables|Default|GetMaxScore) (Variables|Default|GetScore))
        (Variables|Default|SetMaxScore (* (Variables|Default|GetMaxScore) 2.0))
        (Variables|Default|SetScore 0.0 :!pinned true) ; Restart score (UI)
      ))
    (:then_1
      (Actor|DestroyActor _asbp_gem))))

(event Custom|UpdateAnimation
  ;[1 1 1] Run Animation
  (Sprite|SetFlipbook (Variables|Default|GetSprite) (select (AI|Components|NavMovement|IsFalling (Variables|Character|GetCharacterMovement)) "/Game/Images/sprites/Warrior/Individual_Sprite/UptoFall/Warrior_Land.Warrior_Land" (select (> (Math|Vector|VectorLength (Variables|/Script/Engine.MovementComponent|GetVelocity (Variables|Character|GetCharacterMovement))) 0.0) "/Game/Images/sprites/Warrior/Individual_Sprite/Run/Warrior_Run.Warrior_Run" "/Game/Images/sprites/Warrior/Individual_Sprite/idle/Warrior_Idle.Warrior_Idle"))))

(event Custom|UpdateControlRotation
  ;[1 1 1] FaceOrientation
  (Utilities|IsValid (Pawn|GetController)
    (:Is%20Valid
      (Math|Float|CompareFloat (.X (Class|KismetMathLibrary|BreakVector3f (Variables|/Script/Engine.MovementComponent|GetVelocity (Variables|Character|GetCharacterMovement)))) 0.0
        (:>
          (Transformation|SetWorldRotation (Variables|Default|GetSprite) (Math|Rotator|MakeRotator 0.0 0.0 0.0) false false))
        (:<
          (Transformation|SetWorldRotation (Variables|Default|GetSprite) (Math|Rotator|MakeRotator 0.0 0.0 1.8e+02) false false))))))

(event Custom|FindClosestEnemy
  (bind _self self)
  (bind _enemiesinscene (Variables|Default|GetEnemiesInScene))
  (bind _returnvalue (Transformation|GetActorLocation _self))
  (bind _returnvalue_2 (Actor|FindNearestActor _returnvalue _enemiesinscene))
  ;[1 1 1] Find Closest Enemy (Array)
  (Utilities|IsValid _returnvalue_2
    (:Is%20Valid
      (Variables|Default|SetCanShoot true)
      (Transformation|SetWorldRotation (Variables|Default|GetSpawn_projectile) (Math|Rotator|FindLookatRotation (Transformation|GetActorLocation) (Transformation|GetActorLocation _returnvalue_2)) false false) ; Aim
    )
    (:Is%20Not%20Valid
      (Variables|Default|SetCanShoot false))))

(event Custom|Shoot
  ;[1 1 1] Shoot
  (Utilities|FlowControl|Delay (Variables|Default|GetShootFrequency))
  (if (Variables|Default|GetCanShoot)
    (CallFunction|BurstShooting 2)
    (else
      (CallFunction|Shoot))))

(event Custom|BurstShooting
  (params (NumShoots :type Integer))
  (if (> NumShoots 0)
    (Utilities|FlowControl|Delay (Variables|Default|GetBurstCadency))
    (Game|SpawnActorfromClass "/Game/Blueprints/BP_Projectile.BP_Projectile_C" (Transformation|GetWorldTransform (Variables|Default|GetSpawn_projectile)) "Undefined" 0 0)
    (CallFunction|BurstShooting (- NumShoots 1))
    (else
      (CallFunction|Shoot))))

(event Custom|InitializeFindEnemies
  ;[1 1 1] Find Closest Enemy (Array)
  (Utilities|Time|SetTimerbyEvent (delegate Custom|FindClosestEnemy) 0.2 true))

(event EventBeginPlay
  (CallFunction|InitializeFindEnemies)
  (CallFunction|Shoot)
  (bind _actor (CallFunction|FindNearestActorOfClass "/Game/Blueprints/WorldGenerator/BP_WorldGenerator.BP_WorldGenerator_C" "0, 0, 0"))
  (bind _asbp_world_generator (Utilities|Casting|CastToBP_WorldGenerator _actor))
  (Variables|Default|SetWorldGeneratorRef _asbp_world_generator))

(event EventTick
  (params (DeltaSeconds :type Float%20%28single-precision%29))
  (bind _returnvalue (Transformation|GetActorLocation))
  (bind _movementvector (Variables|Default|GetMovementVector))
  (bind _returnvalue_2 (Math|Vector|Normalize _movementvector))
  (bind _returnvalue_3 (* _returnvalue_2 2e+02))
  (bind _returnvalue_4 (+ _returnvalue _returnvalue_3))
  (bind _returnvalue_5 (- _returnvalue_4 "0.000000,0.000000,50.000000"))
  ;[1 1 1] Update()
  (CallFunction|UpdateAnimation)
  (CallFunction|UpdateControlRotation)
  (Transformation|AddLocalRotation (Variables|Default|GetRotatingAttackAxis) (Math|Rotator|MakeRotator 0.0 0.0 (* DeltaSeconds (Variables|Default|GetrotationSpeed))) false false)
  (bind _returnvalue_6 (Collision|MultiLineTraceByChannel _returnvalue_4 _returnvalue_5 "TraceTypeQuery1" false 0 "ForOneFrame"))
  (if (not _returnvalue_6)
    (Default|AddFloor (Variables|Default|GetWorldGeneratorRef) _returnvalue_5)))

(event Game|Damage|EventAnyDamage
  (params (Damage :type Float%20%28single-precision%29) (DamageType :type Damage%20Type%20Object%20Reference) (InstigatedBy :type Controller%20Object%20Reference) (DamageCauser :type Actor%20Object%20Reference))
  ;[1 1 1] Apply damage
  (if (Variables|Default|GetVulnerable)
    ;;[1 1 1] Cooldown
    (Variables|Default|SetVulnerable false)
    (Utilities|FlowControl|Delay (Variables|Default|GetVulnerableCooldown))
    (Variables|Default|SetVulnerable true)
    (Variables|Default|SetHealth (- (Variables|Default|GetHealth) Damage))))

(event Input|ActionEvents|InputActionJump
  (params (Key :type Key%20Structure :default "None"))
  ;[1 1 1] Input
  (:Pressed
    (Character|Jump))
  (:Released
    (Character|StopJumping)))

(event Input|AxisEvents|InputAxisMoveRight
  (params (AxisValue :type Float%20%28single-precision%29))
  ;[1 1 1] Input
  (bind _output_get (Variables|Default|SetMovementVector (Math|Vector|MakeVector AxisValue (* (stale Input|AxisEvents|InputAxisMoveUp AxisValue) -1.0) 0.0)))
  (Pawn|Input|AddMovementInput (Math|Vector|Normalize _output_get) 1.0 false))

(event Input|AxisEvents|InputAxisMoveUp
  (params (AxisValue :type Float%20%28single-precision%29))
  ;[1 1 1] Input
  (bind _output_get (Variables|Default|SetMovementVector (Math|Vector|MakeVector (stale Input|AxisEvents|InputAxisMoveRight AxisValue) (* AxisValue -1.0) 0.0)))
  (Pawn|Input|AddMovementInput (Math|Vector|Normalize _output_get) 1.0 false))

(fn ConstructionScript)

(fn AddEnemytoPool
  (params (EnemyObject :type Actor%20Object%20Reference%20%28by%20ref%29))
  (Utilities|Array|Add (Variables|Default|GetEnemiesInScene) EnemyObject))

(fn RemoveEnemyfromPool
  (params (EnemyToRemove :type Actor%20Object%20Reference%20%28by%20ref%29))
  (Utilities|Array|RemoveItem (Variables|Default|GetEnemiesInScene) EnemyToRemove))