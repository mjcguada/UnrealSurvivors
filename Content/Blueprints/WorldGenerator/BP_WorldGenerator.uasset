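; World generator actor that acts as one floor tile, an instanced static mesh, and can spawn further copies of itself as new tiles.
; AddFloor snaps a hit location to a 1000-unit grid at the actor's height, spawns a tile there and records its mesh in ArrayOfPlanes.
; Its distance check against existing planes reads the element of a loop that is never executed, so it does not scan the array.
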(event EventBeginPlay
  (Utilities|Array|Add (Variables|Default|GetArrayOfPlanes) (Variables|Default|GetInstancedStaticMesh)))

(fn ConstructionScript
  (Components|InstancedStaticMesh|AddInstance (Variables|Default|GetInstancedStaticMesh) (Math|Transform|MakeTransform "0, 0, 0") false))

(fn AddFloor
  (params (HitLocation :type Vector))
  (bind _returnvalue (Transformation|GetActorLocation))
  (bind _returnvalue_2 (Class|KismetMathLibrary|VectorSnappedtoGrid (Math|Vector|MakeVector (.x HitLocation) (.y HitLocation) (.z _returnvalue)) 1e+03))
  (if (> (Math|Vector|Distance2D(Vector) (Math|Conversions|ToVector2D(Vector) _returnvalue_2) (Math|Conversions|ToVector2D(Vector) (Transformation|GetWorldLocation (stale _array_element)))) 1e+02)
    (bind _returnvalue_3 (Game|SpawnActorfromClass "BP_WorldGenerator_C" (Math|Transform|MakeTransform _returnvalue_2 "0, 0, 0" (Transformation|GetActorScale3D)) "Undefined" 0 0))
    (Components|InstancedStaticMesh|AddInstance (Variables|BP_WorldGenerator_C|GetInstancedStaticMesh _returnvalue_3) (Math|Transform|MakeTransform "0, 0, 0") false)
    (Utilities|Array|Add (Variables|Default|GetArrayOfPlanes) (Variables|BP_WorldGenerator_C|GetInstancedStaticMesh _returnvalue_3))))